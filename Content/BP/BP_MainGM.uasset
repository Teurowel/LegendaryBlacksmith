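; Main game manager that holds player progression and economy state: stamina, luck, EXP and rank, money, material inventory and store stock.
; BeginPlay spawns material and item actors from parallel class and key arrays into lookup maps, then seeds empty inventory and random store stock per material.
; Helper functions adjust stats and map counts, and re-roll store stock.
; EXP gains loop through rank-ups, each doubling the threshold and granting stat points.
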(event EventBeginPlay
  (Utilities|FlowControl|Sequence
    (:then_0
      ;[1 1 1] Populate Materail
      (for _index (range 0 (- (Utilities|Array|Length (Variables|Default|GetMaterialClass)) 1))
        (CallFunction|CreateMaterial (Utilities|Array|Get(acopy) (Variables|Default|GetMaterialClass) _index) (Utilities|Array|Get(acopy) (Variables|Default|GetMaterialNames) _index))))
    (:then_1
      ;[1 1 1] Populate Item
      (for _index_2 (range 0 (- (Utilities|Array|Length (Variables|Default|GetItemClass)) 1))
        (CallFunction|CreateItem (Utilities|Array|Get(acopy) (Variables|Default|GetItemClass) _index_2) (Utilities|Array|Get(acopy) (Variables|Default|GetItemKey) _index_2))))
    (:then_2
      ;[1 1 1] Populate Inventory
      (for _array_element (Variables|Default|GetMaterialNames)
        (Utilities|Map|Add (Variables|Default|GetInventory) _array_element 0)))
    (:then_3
      ;[1 1 1] Populate StoreStock
      (for _array_element_2 (Variables|Default|GetMaterialNames)
        (Utilities|Map|Add (Variables|Default|GetStoreStock) _array_element_2 (Math|Random|RandomInteger 10))))))

(event EventTick
  (params (DeltaSeconds :type Float%20%28single-precision%29)))

(fn ConstructionScript)

(fn CreateMaterial
  (params (Class :type BP%20Material%20Class%20Reference) (Key :type String))
  (bind _returnvalue (Game|SpawnActorfromClass Class (Math|Transform|MakeTransform "0, 0, 0" "0, 0, 0" "1,1,1") "Undefined" 0 0))
  (Utilities|Map|Add (Variables|Default|GetMaterials) Key _returnvalue))

(fn CreateItem
  (params (class :type BP%20Item%20Class%20Reference) (Key :type String))
  (bind _returnvalue (Game|SpawnActorfromClass class (Math|Transform|MakeTransform "0, 0, 0" "0, 0, 0" "1,1,1") "Undefined" 0 0))
  (Utilities|Map|Add (Variables|Default|GetItems) Key _returnvalue))

(fn DecreaseStamina
  (params (InSP :type Integer))
  (Variables|Default|SetStaminaCurrent (- (Variables|Default|GetStaminaCurrent) InSP)))

(fn IncreaseEXP
  (params (InEXP :type Integer))
  (bind _output_get (Variables|Default|SetEXP (+ (Variables|Default|GetEXP) InEXP)))
  ;[1 1 1] Keep checking levelup
  (while (LocalVariables|GetWhileLoopBool)
    (if (>= _output_get (Variables|Default|GetMaxEXP))
      (if (not (Utilities|Enum|Equal(Enum) (Variables|Default|GetRank) "NewEnumerator4"))
        (Variables|Default|SetEXP (- (Variables|Default|GetEXP) (Variables|Default|GetMaxEXP)))
        (Variables|Default|SetRank (Utilities|Enum|ByteToEnumEnum_Rank (+ (Variables|Default|GetRank) 1)))
        (Variables|Default|SetMaxEXP (* (Variables|Default|GetMaxEXP) 2))
        (Variables|Default|SetStatPoint (+ (Variables|Default|GetStatPoint) 5)))
      (else
        (LocalVariables|SetWhileLoopBool false)))))

(fn IncreaseMoney
  (params (InMoney :type Integer))
  (Variables|Default|SetMoney (+ (Variables|Default|GetMoney) InMoney)))

(fn DecreaseMoney
  (params (InMoney :type Integer))
  (Variables|Default|SetMoney (- (Variables|Default|GetMoney) InMoney)))

(fn ManipulateInventory
  (params (key :type String) (num :type Integer))
  (LocalVariables|SetTemp (.Value (Utilities|Map|Find (Variables|Default|GetInventory) key)))
  (Utilities|Map|Remove (Variables|Default|GetInventory) key)
  (Utilities|Map|Add (Variables|Default|GetInventory) key (+ num (LocalVariables|GetTemp))))

(fn ManipulateStoreStock
  (params (key :type String) (num :type Integer))
  (LocalVariables|SetTEmp (.Value (Utilities|Map|Find (Variables|Default|GetStoreStock) key)))
  (Utilities|Map|Remove (Variables|Default|GetStoreStock) key)
  (Utilities|Map|Add (Variables|Default|GetStoreStock) key (+ num (LocalVariables|GetTEmp))))

(fn RefreshStoreStock
  (Utilities|Map|Clear (Variables|Default|GetStoreStock))
  (for _array_element (Variables|Default|GetMaterialNames)
    (Utilities|Map|Add (Variables|Default|GetStoreStock) _array_element (Math|Random|RandomInteger 10))))

(fn IncreaseStamina
  (params (InSP :type Integer))
  (Variables|Default|SetStaminaMax (+ (Variables|Default|GetStaminaMax) InSP)))

(fn IncreaseLuck
  (params (InLuck :type Integer))
  (Variables|Default|SetLuck (+ (Variables|Default|GetLuck) InLuck)))